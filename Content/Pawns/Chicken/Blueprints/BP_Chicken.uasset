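; BP_Chicken is the chicken pawn Blueprint, which flashes its body red when hit.
; On BeginPlay it creates a dynamic instance of the body material, caches its Color parameter, and applies it to the animal mesh.
; OnHit restarts a timeline that lerps the Color parameter from the cached color toward a dark red, driven by the timeline's curve.
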(event EventOnHit
  (bind _bodycolor (Timeline|HitTimeline PlayFromStart)
    (:Update
      (Rendering|Material|SetVectorParameterValue (Variables|Default|GetInitialBodyMaterial) "Color" (Math|Color|Lerp(LinearColor) (Variables|Default|GetInitialBodyColor) "(R=0.603922,G=0.094118,B=0.031373,A=1.000000)" _bodycolor) :!class /Script/Engine.MaterialInstanceDynamic))))

(event EventBeginPlay
  (bind _returnvalue (Rendering|Material|CreateDynamicMaterialInstance "/Game/Pawns/Chicken/Materials/MI_Chicken_Body.MI_Chicken_Body" "None" :!class /Script/Engine.KismetMaterialLibrary))
  (Variables|Default|SetInitialBodyMaterial _returnvalue)
  (bind _returnvalue_2 (Rendering|Material|GetVectorParameterValue (Variables|Default|GetInitialBodyMaterial) "Color" :!class /Script/Engine.MaterialInstanceDynamic))
  (Variables|Default|SetInitialBodyColor _returnvalue_2)
  (Rendering|Material|SetMaterial (Variables|Default|GetAnimalMesh) 0 (Variables|Default|GetInitialBodyMaterial)))

(fn ConstructionScript)