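; Chicken-scale logic aside, BP_Coop is a coop construction actor whose appearance reflects its level and build state.
; Initialize swaps the static mesh between the level 1 coop, the level 2 coop, and a level 2 construction mesh used when level 1 is under construction.
; During construction it also reveals the Builder child actor and has that merchant lizard show its hammer.
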(event EventBeginPlay)

(event Collision|EventActorBeginOverlap
  (params (OtherActor :type Actor%20Object%20Reference)))

(event EventTick
  (params (DeltaSeconds :type Float%20%28single-precision%29)))

(event EventInitialize
  (params (CurrentLevel :type Integer) (bIsUnderConstruction :type Boolean))
  (bind _builder (Variables|Default|GetBuilder))
  (switch int CurrentLevel
    (:1
      (if bIsUnderConstruction
        (Components|StaticMesh|SetStaticMesh (Variables|Default|GetStaticMesh) "/Game/Environment/Buildings/ChickenCoops/ChickenCoop2/Misc/S_Coop2_Construction.S_Coop2_Construction")
        (Rendering|SetVisibility _builder true false)
        (bind _asbp_merchant_lizard (Utilities|Casting|CastToBP_MerchantLizard (Variables|/Script/Engine.ChildActorComponent|GetChildActor _builder)))
        (Default|ShowHammer _asbp_merchant_lizard)
        (else
          (Components|StaticMesh|SetStaticMesh (Variables|Default|GetStaticMesh) "/Game/Environment/Buildings/ChickenCoops/ChickenCoop1/Misc/S_Coop.S_Coop"))))
    (:2
      (Components|StaticMesh|SetStaticMesh (Variables|Default|GetStaticMesh) "/Game/Environment/Buildings/ChickenCoops/ChickenCoop2/Misc/S_Coop2.S_Coop2"))))

(fn ConstructionScript)