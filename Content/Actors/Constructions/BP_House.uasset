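; BP_House is a house construction actor whose look reflects its level and whether it is being built.
; Initialize swaps the static mesh to match level one, level two, or the level-two construction stage shown during a level-one upgrade.
; During that upgrade it also reveals the Builder child actor, a merchant lizard that shows its hammer and loops a building animation.
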(event EventBeginPlay)

(event Collision|EventActorBeginOverlap
  (params (OtherActor :type Actor%20Object%20Reference)))

(event EventTick
  (params (DeltaSeconds :type Float%20%28single-precision%29)))

(event EventInitialize
  (params (CurrentLevel :type Integer) (bIsUnderConstruction :type Boolean))
  (bind _builder (Variables|Default|GetBuilder))
  (switch int CurrentLevel
    (:1
      (if bIsUnderConstruction
        (Components|StaticMesh|SetStaticMesh (Variables|Default|GetStaticMesh) "/Game/Environment/Buildings/House/House2/Misc/S_House2_Construction.S_House2_Construction")
        (Rendering|SetVisibility _builder true false)
        (bind _asbp_merchant_lizard (Utilities|Casting|CastToBP_MerchantLizard (Variables|/Script/Engine.ChildActorComponent|GetChildActor _builder)))
        (Default|ShowHammer _asbp_merchant_lizard)
        (Components|Animation|PlayAnimation (Variables|/Script/Engine.Character|GetMesh _asbp_merchant_lizard) "/Game/Characters/MerchantLizard/Animations/MerchantiLizard_Building2.MerchantiLizard_Building2" true)
        (else
          (Components|StaticMesh|SetStaticMesh (Variables|Default|GetStaticMesh) "/Game/Environment/Buildings/House/House1/Misc/S_House1.S_House1"))))
    (:2
      (Components|StaticMesh|SetStaticMesh (Variables|Default|GetStaticMesh) "/Game/Environment/Buildings/House/House2/Misc/S_House2.S_House2"))))

(fn ConstructionScript)