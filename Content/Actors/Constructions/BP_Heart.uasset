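; BP_Heart is a construction actor for a heart structure on a base, with visuals that follow its build level.
; Initialize shows construction meshes at level 0 while building and clears them otherwise, then uses finished meshes at level 1.
; The finished heart spins through a RotatingMovement component, while FloatTimeline offsets its height from the location cached at BeginPlay.
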(event EventBeginPlay
  (Variables|Default|SetInitialHeartLocation (Variables|/Script/Engine.SceneComponent|GetRelativeLocation (Variables|Default|GetHeart))))

(event Collision|EventActorBeginOverlap
  (params (OtherActor :type Actor%20Object%20Reference)))

(event EventTick
  (params (DeltaSeconds :type Float%20%28single-precision%29)))

(event EventInitialize
  (params (CurrentLevel :type Integer) (bIsUnderConstruction :type Boolean))
  (switch int CurrentLevel
    (:0
      (if bIsUnderConstruction
        (Components|StaticMesh|SetStaticMesh (Variables|Default|GetBase) "/Game/Environment/Buildings/Heart/Misc/S_HeartBase_Construction.S_HeartBase_Construction")
        (Components|StaticMesh|SetStaticMesh (Variables|Default|GetHeart) "/Game/Environment/Buildings/Heart/Misc/S_Heart_Construction.S_Heart_Construction")
        (Transformation|SetRelativeLocation (Variables|Default|GetHeart) "0, 0,91.666794" false false)
        (else
          (Components|StaticMesh|SetStaticMesh (Variables|Default|GetBase) 0)
          (Components|StaticMesh|SetStaticMesh (Variables|Default|GetHeart) 0))))
    (:1
      (Components|StaticMesh|SetStaticMesh (Variables|Default|GetBase) "/Game/Environment/Buildings/Heart/Misc/S_HeartBase.S_HeartBase")
      (Components|StaticMesh|SetStaticMesh (Variables|Default|GetHeart) "/Game/Environment/Buildings/Heart/Misc/S_Heart.S_Heart")
      (Variables|/Script/Engine.RotatingMovementComponent|SetRotationRate (Variables|Default|GetRotatingMovement) (Variables|Default|GetRotationRate))
      (Components|Movement|SetUpdatedComponent (Variables|Default|GetRotatingMovement) (Variables|Default|GetHeart))
      (Components|Activation|Activate (Variables|Default|GetRotatingMovement) false)
      (bind _verticaloffset (Timeline|FloatTimeline PlayFromStart)
        (:Update
          (Transformation|SetRelativeLocation (Variables|Default|GetHeart) (+ (Variables|Default|GetInitialHeartLocation) (Math|Vector|MakeVector 0.0 0.0 (* _verticaloffset (Variables|Default|GetFloatOffset)))) false false))))))

(fn ConstructionScript)