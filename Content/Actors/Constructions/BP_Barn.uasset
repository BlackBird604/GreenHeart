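; Barn construction actor whose appearance reflects its level and whether it is being built.
; Initialize switches the static mesh between the level 1 barn, the level 2 barn and the upgrade construction site, which only level 1 can show.
; During construction it also reveals the Builder child actor, a merchant lizard holding a hammer, and enables query-only collision on BuilderBox.
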(event EventBeginPlay)

(event Collision|EventActorBeginOverlap
  (params (OtherActor :type Actor%20Object%20Reference)))

(event EventTick
  (params (DeltaSeconds :type Float%20%28single-precision%29)))

(event EventInitialize
  (params (CurrentLevel :type Integer) (bIsUnderConstruction :type Boolean))
  (bind _builder (Variables|Default|GetBuilder))
  (switch int CurrentLevel
    (:1
      (if bIsUnderConstruction
        (Components|StaticMesh|SetStaticMesh (Variables|Default|GetStaticMesh) "/Game/Environment/Buildings/Barn/Barn2/S_Barn2_Construction.S_Barn2_Construction")
        (Rendering|SetVisibility _builder true false)
        (bind _asbp_merchant_lizard (Utilities|Casting|CastToBP_MerchantLizard (Variables|/Script/Engine.ChildActorComponent|GetChildActor _builder)))
        (Default|ShowHammer _asbp_merchant_lizard)
        (Collision|SetCollisionEnabled (Variables|Default|GetBuilderBox) "QueryOnly")
        (else
          (Components|StaticMesh|SetStaticMesh (Variables|Default|GetStaticMesh) "/Game/Environment/Buildings/Barn/Barn1/Misc/S_Barn.S_Barn"))))
    (:2
      (Components|StaticMesh|SetStaticMesh (Variables|Default|GetStaticMesh) "/Game/Environment/Buildings/Barn/Barn2/S_Barn2.S_Barn2"))))

(fn ConstructionScript)