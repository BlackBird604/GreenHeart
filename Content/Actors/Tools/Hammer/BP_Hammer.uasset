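; Hammer tool actor whose head changes appearance by level.
; The SetupMaterial event switches on Level across four stages, swapping the materials in two head slots of ToolMesh for that stage's pair.
; The Blueprint holds no other logic, and its construction script is empty.
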(event EventSetupMaterial
  (params (Level :type Integer))
  (switch int Level
    (:0
      (Rendering|Material|SetMaterial (Variables|Default|GetToolMesh) 1 "/Game/Actors/Tools/Hammer/Materials/MI_HammerHead01_Stage1.MI_HammerHead01_Stage1")
      (Rendering|Material|SetMaterial (Variables|Default|GetToolMesh) 2 "/Game/Actors/Tools/Hammer/Materials/MI_HammerHead02_Stage1.MI_HammerHead02_Stage1"))
    (:1
      (Rendering|Material|SetMaterial (Variables|Default|GetToolMesh) 1 "/Game/Actors/Tools/Hammer/Materials/MI_HammerHead01_Stage2.MI_HammerHead01_Stage2")
      (Rendering|Material|SetMaterial (Variables|Default|GetToolMesh) 2 "/Game/Actors/Tools/Hammer/Materials/MI_HammerHead02_Stage2.MI_HammerHead02_Stage2"))
    (:2
      (Rendering|Material|SetMaterial (Variables|Default|GetToolMesh) 1 "/Game/Actors/Tools/Hammer/Materials/MI_HammerHead01_Stage3.MI_HammerHead01_Stage3")
      (Rendering|Material|SetMaterial (Variables|Default|GetToolMesh) 2 "/Game/Actors/Tools/Hammer/Materials/MI_HammerHead02_Stage3.MI_HammerHead02_Stage3"))
    (:3
      (Rendering|Material|SetMaterial (Variables|Default|GetToolMesh) 1 "/Game/Actors/Tools/Hammer/Materials/MI_HammerHead01_Stage4.MI_HammerHead01_Stage4")
      (Rendering|Material|SetMaterial (Variables|Default|GetToolMesh) 2 "/Game/Actors/Tools/Hammer/Materials/MI_HammerHead02_Stage4.MI_HammerHead02_Stage4"))))

(fn ConstructionScript)