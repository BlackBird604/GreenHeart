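; BP_SunPosition is an actor that drives the farming game's sun and sky lighting from the in-game clock.
; On BeginPlay it binds to the FarmingGameMode's time-updated event, storing each new hour and minute and calling UpdateSun.
; It scrubs a timeline to the normalized fraction of the day, whose curves set directional light and skylight intensity on update.
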(event Custom|OnTimeUpdated
  (params (NewHour :type Integer) (NewMinute :type Integer))
  (Variables|Default|SetHours NewHour)
  (Variables|Default|SetMinutes NewMinute)
  (CallFunction|UpdateSun)
  (bind (_direction _directionallightintansity _skylightintensity) (Timeline|LightIntensityTimeline SetNewTime)
    (:Update
      (Rendering|Components|Light|SetIntensity (Variables|/Script/Engine.Light|GetLightComponent (Variables|Default|GetDirectionalLight)) _directionallightintansity)
      (Rendering|Components|Light|SetIntensity (Variables|/Script/Engine.SkyLight|GetLightComponent (Variables|Default|GetSkyLight)) _skylightintensity))))

(event EventBeginPlay
  (bind _asfarming_game_mode (Utilities|Casting|CastToFarmingGameMode (Game|GetGameMode)))
  (EventDispatchers|BindEventtoOnTimeUpdated _asfarming_game_mode (delegate Custom|OnTimeUpdated)))

(fn ConstructionScript
  (|CallParentFunction))