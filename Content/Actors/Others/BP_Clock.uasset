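; BP_Clock is a clock actor whose hands show the in-game time of the farming game.
; On BeginPlay it binds to the FarmingGameMode's time-updated event.
; Each update rotates the hour and minute pivots on pitch, with the hour hand advancing smoothly with minutes on a 12-hour dial.
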(event Custom|OnTimeUpdated
  (params (NewHour :type Integer) (NewMinute :type Integer))
  (Transformation|SetRelativeRotation (Variables|Default|GetHourPivot) (Math|Rotator|MakeRotator 0.0 (/ (Math|Conversions|ToFloat(Integer) (+ (* (Math|Integer|%(Integer) NewHour 12) 60) NewMinute)) -2.0) 0.0) false false)
  (Transformation|SetRelativeRotation (Variables|Default|GetMinutePivot) (Math|Rotator|MakeRotator 0.0 (Math|Conversions|ToFloat(Integer) (* NewMinute -6)) 0.0) false false))

(event EventBeginPlay
  (bind _asfarming_game_mode (Utilities|Casting|CastToFarmingGameMode (Game|GetGameMode)))
  (EventDispatchers|BindEventtoOnTimeUpdated _asfarming_game_mode (delegate Custom|OnTimeUpdated)))

(fn ConstructionScript)