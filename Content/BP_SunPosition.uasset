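; Sun position actor that keeps the sun in step with the farming game's clock.
; On BeginPlay it binds to the FarmingGameMode time-updated event, so it needs no Tick logic.
; Each update stores the new hour and minute, then calls UpdateSun, whose logic is not defined in these graphs.
; A leftover delay-based clock that advances minutes and hours is disconnected and never runs.
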(event Custom|OnTimeUpdated
  (params (NewHour :type Integer) (NewMinute :type Integer))
  (Variables|Default|SetHours NewHour)
  (Variables|Default|SetMinutes NewMinute)
  (CallFunction|UpdateSun))

(event EventBeginPlay
  (bind _asfarming_game_mode (Utilities|Casting|CastToFarmingGameMode (Game|GetGameMode)))
  (EventDispatchers|BindEventtoOnTimeUpdated _asfarming_game_mode (delegate Custom|OnTimeUpdated)))

(event Collision|EventActorBeginOverlap
  (params (OtherActor :type Actor%20Object%20Reference)))

(event EventTick
  (params (DeltaSeconds :type Float%20%28single-precision%29)))

(fn ConstructionScript
  (|CallParentFunction))